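; Cartoon water lake Blueprint that exposes the look of the water surface as editable variables.
; Its Construction Script creates a dynamic material instance on the CartoonWater component from CartoonWaterReference.
; Collapsed graphs then push the variables into that instance, grouped by color, displacement, foam, fresnel, highlight, depth, normals and global settings such as wave speed and direction.
; The fresnel variables drive material parameters named Fog.
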(fn `UserConstructionScript`
  (bind _cartoonwaterinstance (`self.CartoonWaterInstance`))
  (bind _returnvalue (`PrimitiveComponent.CreateDynamicMaterialInstance` (`self.CartoonWater`) 0 (`self.Cartoon Water Reference`) "None"))
  (set `self.CartoonWaterInstance` _returnvalue)
  (`MaterialInstanceDynamic.SetVectorParameterValue` _cartoonwaterinstance "Water Color" (`self.Primary Water Color`)) ; Set the primary water color
  (`MaterialInstanceDynamic.SetVectorParameterValue` _cartoonwaterinstance "Deepwater Color" (`self.Deep Water Color`)) ; Set the deep water color
  (`MaterialInstanceDynamic.SetVectorParameterValue` _cartoonwaterinstance "Fog Color" (`self.Water Fresnel Color`)) ; Set the water's fresnel color
  (`MaterialInstanceDynamic.SetVectorParameterValue` _cartoonwaterinstance "Intersection Color" (`self.Intersection Color`)) ; Set the intersection color
  (`MaterialInstanceDynamic.SetScalarParameterValue` _cartoonwaterinstance "Displacement Tiling" (`self.Wave Tiling`)) ; Set the wave tiling
  (`MaterialInstanceDynamic.SetScalarParameterValue` _cartoonwaterinstance "Wave Strength" (`self.Wave Strength`)) ; Set the wave strength
  (`MaterialInstanceDynamic.SetScalarParameterValue` _cartoonwaterinstance "Foam Tiling" (`self.Foam Tiling`)) ; Set the foam tiling
  (`MaterialInstanceDynamic.SetScalarParameterValue` _cartoonwaterinstance "Intersection Size" (`self.Foam Intersection Size`)) ; Set the foam intersection size
  (`MaterialInstanceDynamic.SetScalarParameterValue` _cartoonwaterinstance "Intersection Strength" (`self.Foam Strength`)) ; Set the foam strength
  (`MaterialInstanceDynamic.SetScalarParameterValue` _cartoonwaterinstance "Intersection Visibility" (`self.Foam Transparency`)) ; Set the foam transparency
  (`MaterialInstanceDynamic.SetScalarParameterValue` _cartoonwaterinstance "Fog Slope" (`self.Fresnel Slope`)) ; Set the fresnel slope
  (`MaterialInstanceDynamic.SetScalarParameterValue` _cartoonwaterinstance "Fog Strength" (`self.Fresnel Strength`)) ; Set the fresnel strength
  (`MaterialInstanceDynamic.SetScalarParameterValue` _cartoonwaterinstance "Fog Visibility" (`self.Fresnel Transparency`)) ; Set the fresnel transparency
  (`MaterialInstanceDynamic.SetScalarParameterValue` _cartoonwaterinstance "Surface Highlight Tiling" (`self.Surface Highlight Tiling`)) ; Set the surface highlight tiling
  (`MaterialInstanceDynamic.SetScalarParameterValue` _cartoonwaterinstance "Surface Highlight" (`self.Surface Highlight Strength`)) ; Set the surface highlight strength
  (`MaterialInstanceDynamic.SetScalarParameterValue` _cartoonwaterinstance "Surface Highlight Size" (`self.Surface Highlight Size`)) ; Set the surface highlight size
  (`MaterialInstanceDynamic.SetScalarParameterValue` _cartoonwaterinstance "Water Depth" (`self.Water Depth`)) ; Set the water depth
  (`MaterialInstanceDynamic.SetScalarParameterValue` _cartoonwaterinstance "Water Depth Power" (`self.Water Depth Power`)) ; Set the water depth power
  (`MaterialInstanceDynamic.SetScalarParameterValue` _cartoonwaterinstance "Water Height" (`self.Water Height`)) ; Set the water height
  (`MaterialInstanceDynamic.SetScalarParameterValue` _cartoonwaterinstance "NormalTiling" (`self.Normal Tiling`)) ; Set the normal Tiling
  (`MaterialInstanceDynamic.SetScalarParameterValue` _cartoonwaterinstance "Normal Intensity" (`self.Normal Strength`)) ; Set the normal strength
  (`MaterialInstanceDynamic.SetScalarParameterValue` _cartoonwaterinstance "Wave Speed" (`self.Wave Speed`)) ; Set the wave speed
  (`MaterialInstanceDynamic.SetScalarParameterValue` _cartoonwaterinstance "Glossiness" (`self.Glossines`)) ; Set the glossines
  (`MaterialInstanceDynamic.SetScalarParameterValue` _cartoonwaterinstance "Refraction" (`self.Refraction`)) ; Set the refraction
  (`MaterialInstanceDynamic.SetScalarParameterValue` _cartoonwaterinstance "Transparency" (`self.Transparency`)) ; set the overal water transparency
  (`MaterialInstanceDynamic.SetScalarParameterValue` _cartoonwaterinstance "X Direction" (`self.X Direction`)) ; Set the direction of X
  (`MaterialInstanceDynamic.SetScalarParameterValue` _cartoonwaterinstance "Y Direction" (`self.Y Direction`)))